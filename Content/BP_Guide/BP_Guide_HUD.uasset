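; BP_Guide_HUD is the guide game's HUD, showing score, level and time on screen.
; On BeginPlay it caches the game mode cast to BP_Guide_GameMode.
; Each DrawHUD call reads that game mode's values and draws them as colored canvas text at fixed screen positions.
; When the game mode's GameOver flag is set, it also draws a game-over message with a Press Enter prompt.
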(event `self.ReceiveBeginPlay`
  (bind _asbp_guide_game_mode (cast `/Game/BP_Guide/BP_Guide_GameMode` (`GameplayStatics.GetGameMode`)))
  (set `self.My Guide Game Mode` _asbp_guide_game_mode))

(event `self.ReceiveDrawHUD`
  (params (SizeX :type Integer) (SizeY :type Integer))
  ;[1 1 1] Draw HUD
  ;;[1 1 1] Score
  (`self.DrawText` (`KismetStringLibrary.BuildString_Int` "Score:" "" (`/Game/BP_Guide/BP_Guide_GameMode.Score` (`self.My Guide Game Mode`))) (struct :`R` 0.648891 :`G` 0.708333 :`B` 0.110495 :`A` 1.0) 10.0 10.0 null 3.0)
  ;;[1 1 1] Level
  (`self.DrawText` (`KismetStringLibrary.BuildString_Int` "Level:" "" (`/Game/BP_Guide/BP_Guide_GameMode.Level` (`self.My Guide Game Mode`))) (struct :`R` 1.0 :`B` 0.028928 :`A` 1.0) 300.0 10.0 null 3.0)
  ;;[1 1 1] Time
  (`self.DrawText` (`KismetStringLibrary.BuildString_Int` "Time:" "" (`/Game/BP_Guide/BP_Guide_GameMode.Time` (`self.My Guide Game Mode`))) (struct :`G` 0.35691 :`B` 1.0 :`A` 1.0) 550.0 10.0 null 3.0)
  (if (`/Game/BP_Guide/BP_Guide_GameMode.GameOver` (`self.My Guide Game Mode`))
    (`self.DrawText` "GAME OVER!" (struct :`R` 1.0 :`A` 1.0) 400.0 200.0 null 3.0)
    (`self.DrawText` "Press Enter" (struct :`R` 1.0 :`A` 1.0) 400.0 400.0 null 3.0)))

(fn `UserConstructionScript`)